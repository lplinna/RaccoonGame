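; BP_RaccoonPlayer is the player raccoon Blueprint, picking a directional flipbook animation every Tick.
; The dominant MoveForward or MoveRight input chooses the axis, and velocity sign on X or Y selects Forward/Backward or Left/Right.
; Idle shows only on the Y branch at zero velocity, as the X branch's idle check is left unconnected.
; Each Tick also prints the chosen flipbook's name for debugging.
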(event `self.ReceiveBeginPlay`)

(event `self.ReceiveTick`
  (params (DeltaSeconds :type "Float (single-precision)"))
  (bind (_returnvalue_x _returnvalue_y) (`KismetMathLibrary.BreakVector` (`self.GetVelocity` (`ActorComponent.GetOwner` (`self.CapsuleComponent`)))))
  (bind _returnvalue (select `bool` (== 0.0 _returnvalue_y) :`false` (select `bool` (> _returnvalue_y 0.0) :`false` (`self.leftAnimation`) :`true` (`self.rightAnimation`)) :`true` (`self.IdleAnimation`)))
  (bind _returnvalue_2 (select `bool` false :`false` (select `bool` (> _returnvalue_x 0.0) :`false` (`self.ForwardAnimation`) :`true` (`self.BackwardAnimation`)) :`true` (`self.IdleAnimation`)))
  (if (> (`KismetMathLibrary.Abs` (`self.GetInputAxisValue`)) (`KismetMathLibrary.Abs` (`self.GetInputAxisValue`)))
    (`PaperFlipbookComponent.SetFlipbook` (`self.PaperFlipbook`) _returnvalue_2)
    (`KismetSystemLibrary.PrintString` (`KismetSystemLibrary.GetDisplayName` _returnvalue_2))
    (else
      (`PaperFlipbookComponent.SetFlipbook` (`self.PaperFlipbook`) _returnvalue)
      (`KismetSystemLibrary.PrintString` (`KismetSystemLibrary.GetDisplayName` _returnvalue)))))

(fn `UserConstructionScript`)